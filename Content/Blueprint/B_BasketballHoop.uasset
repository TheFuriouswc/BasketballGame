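; Basketball hoop actor that awards a score when a Basketball passes into its ScoreCapsule trigger.
; On BeginPlay it caches the BasketballGameGameStateBase, then passes it with the ball to ServerAddScore on overlap.
; A DoOnce gate blocks repeat scoring until a Basketball ends its overlap with the capsule, which resets it.
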(event `self.ReceiveBeginPlay`
  (bind _asbasketball_game_game_state_base (cast `BasketballGameGameStateBase` (`GameplayStatics.GetGameState`))
    (:`then`
      (set `self.GameState` _asbasketball_game_game_state_base))
    (:`CastFailed`
      (`KismetSystemLibrary.PrintString` "Cast failed for game stae"))))

(event `self.ScoreCapsule.OnComponentBeginOverlap`
  (params (OverlappedComponent :type "PrimitiveComponent Object Reference") (OtherActor :type "Actor Object Reference") (OtherComp :type "PrimitiveComponent Object Reference") (OtherBodyIndex :type Integer) (bFromSweep :type Boolean) (SweepResult :type "HitResult Structure (by ref)"))
  (bind _asbasketball (cast `Basketball` OtherActor)
    (:`then`
      (`/Engine/EditorBlueprintResources/StandardMacros.DoOnce` false :!label _label
        (:`Completed`
          (`self.Server_AddScore` _asbasketball (`self.GameState`)))))
    (:`CastFailed`
      (`KismetSystemLibrary.PrintString` "Cast failed"))))

(event `self.ScoreCapsule.OnComponentEndOverlap`
  (params (OverlappedComponent :type "PrimitiveComponent Object Reference") (OtherActor :type "Actor Object Reference") (OtherComp :type "PrimitiveComponent Object Reference") (OtherBodyIndex :type Integer))
  (cast `Basketball` OtherActor
    (:`then`
      (goto _label :!via `Reset`))
    (:`CastFailed`
      (`KismetSystemLibrary.PrintString` "Cast failed"))))

(fn `UserConstructionScript`)