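; BP_FireBallPowerUp is a power-up Blueprint that sets a player's held basketball on fire.
; Its UsePower event receives a player reference and, if that player has a basketball, sets OnFire on the player's basketball reference and prints a debug message.
; The default BeginPlay, overlap and Tick events are disabled, and the graph contains no logic to switch the fire state back off.
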(event `/Game/Blueprint/BlueprintInterface/BPI_PowerUp.UsePower`
  (params (PlayerRef :type "/Game/ThirdPerson/Blueprints/BP_BasketBallPlayer Object Reference") (ControllerRef :type "PlayerController Object Reference"))
  (if (`BasketballGameCharacter.bHasBasketball` PlayerRef)
    (set `Basketball.OnFire` true (`BasketballGameCharacter.BasketballRef` PlayerRef))
    (`KismetSystemLibrary.PrintString` "Fire ball On")))

(fn `UserConstructionScript`
  (`parent.UserConstructionScript`))