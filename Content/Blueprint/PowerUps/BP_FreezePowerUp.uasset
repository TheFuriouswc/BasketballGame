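; BP_FreezePowerUp is a power-up that slows every BP_BasketBallPlayer with BulletTime while exempting the player who used it.
; UsePower stores that player and triggers Mulit_SetBulletTime, which halves each player's time scale, then restores the user's to normal.
; A delayed timeline drives the reset, but both sit inside the loop, so its updates reach only the last player iterated.
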(event `/Game/Blueprint/BlueprintInterface/BPI_PowerUp.UsePower`
  (params (PlayerRef :type "/Game/ThirdPerson/Blueprints/BP_BasketBallPlayer Object Reference") (ControllerRef :type "PlayerController Object Reference"))
  (set `self.Player Ref` PlayerRef)
  (`self.Mulit_SetBulletTime`))

(event `Mulit_SetBulletTime`
  (bind _outactors (`GameplayStatics.GetAllActorsOfClass` "/Game/ThirdPerson/Blueprints/BP_BasketBallPlayer.BP_BasketBallPlayer_C"))
  (for _array_element _outactors
    (`/Game/ThirdPerson/Blueprints/BP_BasketBallPlayer.BulletTime` _array_element 0.5)
    (`KismetSystemLibrary.Delay` 4.0)
    (bind (_direction _time_dilation) (`Timeline|ResetBulletTimeTimeLine` :!via `PlayFromStart`)
      (:`Update`
        (`/Game/ThirdPerson/Blueprints/BP_BasketBallPlayer.BulletTime` _array_element _time_dilation)
        (`KismetSystemLibrary.PrintString` "Time reset"))))
  (`/Game/ThirdPerson/Blueprints/BP_BasketBallPlayer.BulletTime` (`self.Player Ref`) 1.0)
  (`KismetSystemLibrary.Delay` 4.0))

(fn `UserConstructionScript`
  (`parent.UserConstructionScript`))